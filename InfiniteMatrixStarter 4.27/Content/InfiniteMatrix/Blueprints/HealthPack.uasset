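; HealthPack is a pickup actor that restores player health when overlapped.
; A BP_Player overlap calls IncrementHealth on that player, then destroys the pack.
; A Bullet overlap destroys the bullet and also heals the pawn at player index 0, so the pack can be collected by shooting it.
; A separate DestroyHealthPack function simply destroys the actor.
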(event `self.ReceiveActorBeginOverlap`
  (params (OtherActor :type "Actor Object Reference"))
  (bind _asbp_player (cast `/Game/InfiniteMatrix/Blueprints/BP_Player` OtherActor)
    (:`then`
      (`/Game/InfiniteMatrix/Blueprints/BP_Player.IncrementHealth` _asbp_player)
      (`self.K2_DestroyActor`))
    (:`CastFailed`
      (bind _asbullet (cast `/Game/InfiniteMatrix/Blueprints/Bullet` OtherActor))
      (`self.K2_DestroyActor` _asbullet)
      (bind _asbp_player_2 (cast `/Game/InfiniteMatrix/Blueprints/BP_Player` (`GameplayStatics.GetPlayerPawn` 0)))
      (`/Game/InfiniteMatrix/Blueprints/BP_Player.IncrementHealth` _asbp_player_2)
      (`self.K2_DestroyActor`))))

(event `self.Collider.OnComponentHit`
  (params (HitComponent :type "PrimitiveComponent Object Reference") (OtherActor :type "Actor Object Reference") (OtherComp :type "PrimitiveComponent Object Reference") (NormalImpulse :type "Vector Structure") (Hit :type "HitResult Structure (by ref)")))

(fn `Destroy HealthPack`
  (`self.K2_DestroyActor`))

(fn `UserConstructionScript`)